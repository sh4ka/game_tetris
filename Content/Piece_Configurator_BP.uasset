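; Piece configurator for a Tetris-style game that picks one of the seven tetromino shapes and returns its block layout.
; ReturnRandomPiece samples a random entry among the first hundred of the supplied noise map and maps its value through threshold bands to a shape.
; Each shape function builds PieceConfig from four hardcoded 2D grid offsets.
; Construction and event graphs are empty, so it only serves these functions.
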(event EventBeginPlay)

(event Collision|EventActorBeginOverlap
  (params (OtherActor :type Actor%20Object%20Reference)))

(event EventTick
  (params (DeltaSeconds :type Float%20%28single-precision%29)))

(fn ConstructionScript)

(fn ReturnRandomPiece
  (params (NoiseMap :type Array%20of%20Integers))
  (bind _output_get (LocalVariables|SetNoise NoiseMap))
  (bind _output_get_2 (LocalVariables|SetRandNumber (Utilities|Array|Get(acopy) _output_get (Math|Random|RandomIntegerinRange 0 99))))
  (if (< _output_get_2 13)
    (bind _piece_config (CallFunction|ReturnStripe))
    (LocalVariables|SetResultingPiece _piece_config)
    (return (LocalVariables|GetResultingPiece))
    (elif (< _output_get_2 27)
      (bind _piece_config_2 (CallFunction|ReturnBox))
      (LocalVariables|SetResultingPiece _piece_config_2)
      (return (LocalVariables|GetResultingPiece))
      (elif (< _output_get_2 41)
        (bind _piece_config_3 (CallFunction|ReturnZ))
        (LocalVariables|SetResultingPiece _piece_config_3)
        (return (LocalVariables|GetResultingPiece))
        (elif (< _output_get_2 55)
          (bind _piece_config_4 (CallFunction|ReturnS))
          (LocalVariables|SetResultingPiece _piece_config_4)
          (return (LocalVariables|GetResultingPiece))
          (elif (< _output_get_2 69)
            (bind _piece_config_5 (CallFunction|ReturnL))
            (LocalVariables|SetResultingPiece _piece_config_5)
            (return (LocalVariables|GetResultingPiece))
            (elif (< _output_get_2 85)
              (bind _piece_config_6 (CallFunction|ReturnJ))
              (LocalVariables|SetResultingPiece _piece_config_6)
              (return (LocalVariables|GetResultingPiece))
              (elif (< _output_get_2 100)
                (bind _piece_config_7 (CallFunction|ReturnT))
                (LocalVariables|SetResultingPiece _piece_config_7)
                (return (LocalVariables|GetResultingPiece))
                (else
                  (Development|PrintString "Error getting random piece"))))))))))

(fn ReturnStripe
  (Utilities|FlowControl|Sequence
    (:then_0
      (Utilities|Array|Add (LocalVariables|GetPieceConfig) (Math|Vector2D|MakeVector2D 1.0 0.0)))
    (:then_1
      (Utilities|Array|Add (LocalVariables|GetPieceConfig) (Math|Vector2D|MakeVector2D 1.0 1.0)))
    (:then_2
      (Utilities|Array|Add (LocalVariables|GetPieceConfig) (Math|Vector2D|MakeVector2D 1.0 2.0)))
    (:then_3
      (Utilities|Array|Add (LocalVariables|GetPieceConfig) (Math|Vector2D|MakeVector2D 1.0 3.0)))
    (:then_4
      (return (LocalVariables|GetPieceConfig)))))

(fn ReturnBox
  (Utilities|FlowControl|Sequence
    (:then_0
      (Utilities|Array|Add (LocalVariables|GetPieceConfig) (Math|Vector2D|MakeVector2D 1.0 0.0)))
    (:then_1
      (Utilities|Array|Add (LocalVariables|GetPieceConfig) (Math|Vector2D|MakeVector2D 2.0 0.0)))
    (:then_2
      (Utilities|Array|Add (LocalVariables|GetPieceConfig) (Math|Vector2D|MakeVector2D 1.0 1.0)))
    (:then_3
      (Utilities|Array|Add (LocalVariables|GetPieceConfig) (Math|Vector2D|MakeVector2D 2.0 1.0)))
    (:then_4
      (return (LocalVariables|GetPieceConfig)))))

(fn ReturnZ
  (Utilities|FlowControl|Sequence
    (:then_0
      (Utilities|Array|Add (LocalVariables|GetPieceConfig) (Math|Vector2D|MakeVector2D 1.0 1.0)))
    (:then_1
      (Utilities|Array|Add (LocalVariables|GetPieceConfig) (Math|Vector2D|MakeVector2D 2.0 1.0)))
    (:then_2
      (Utilities|Array|Add (LocalVariables|GetPieceConfig) (Math|Vector2D|MakeVector2D 2.0 0.0)))
    (:then_3
      (Utilities|Array|Add (LocalVariables|GetPieceConfig) (Math|Vector2D|MakeVector2D 3.0 0.0)))
    (:then_4
      (return (LocalVariables|GetPieceConfig)))))

(fn ReturnS
  (Utilities|FlowControl|Sequence
    (:then_0
      (Utilities|Array|Add (LocalVariables|GetPieceConfig) (Math|Vector2D|MakeVector2D 0.0 0.0)))
    (:then_1
      (Utilities|Array|Add (LocalVariables|GetPieceConfig) (Math|Vector2D|MakeVector2D 1.0 0.0)))
    (:then_2
      (Utilities|Array|Add (LocalVariables|GetPieceConfig) (Math|Vector2D|MakeVector2D 1.0 1.0)))
    (:then_3
      (Utilities|Array|Add (LocalVariables|GetPieceConfig) (Math|Vector2D|MakeVector2D 2.0 1.0)))
    (:then_4
      (return (LocalVariables|GetPieceConfig)))))

(fn ReturnL
  (Utilities|FlowControl|Sequence
    (:then_0
      (Utilities|Array|Add (LocalVariables|GetPieceConfig) (Math|Vector2D|MakeVector2D 1.0 2.0)))
    (:then_1
      (Utilities|Array|Add (LocalVariables|GetPieceConfig) (Math|Vector2D|MakeVector2D 1.0 1.0)))
    (:then_2
      (Utilities|Array|Add (LocalVariables|GetPieceConfig) (Math|Vector2D|MakeVector2D 1.0 0.0)))
    (:then_3
      (Utilities|Array|Add (LocalVariables|GetPieceConfig) (Math|Vector2D|MakeVector2D 2.0 0.0)))
    (:then_4
      (return (LocalVariables|GetPieceConfig)))))

(fn ReturnJ
  (Utilities|FlowControl|Sequence
    (:then_0
      (Utilities|Array|Add (LocalVariables|GetPieceConfig) (Math|Vector2D|MakeVector2D 1.0 0.0)))
    (:then_1
      (Utilities|Array|Add (LocalVariables|GetPieceConfig) (Math|Vector2D|MakeVector2D 2.0 0.0)))
    (:then_2
      (Utilities|Array|Add (LocalVariables|GetPieceConfig) (Math|Vector2D|MakeVector2D 2.0 1.0)))
    (:then_3
      (Utilities|Array|Add (LocalVariables|GetPieceConfig) (Math|Vector2D|MakeVector2D 2.0 2.0)))
    (:then_4
      (return (LocalVariables|GetPieceConfig)))))

(fn ReturnT
  (Utilities|FlowControl|Sequence
    (:then_0
      (Utilities|Array|Add (LocalVariables|GetPieceConfig) (Math|Vector2D|MakeVector2D 1.0 0.0)))
    (:then_1
      (Utilities|Array|Add (LocalVariables|GetPieceConfig) (Math|Vector2D|MakeVector2D 2.0 0.0)))
    (:then_2
      (Utilities|Array|Add (LocalVariables|GetPieceConfig) (Math|Vector2D|MakeVector2D 3.0 0.0)))
    (:then_3
      (Utilities|Array|Add (LocalVariables|GetPieceConfig) (Math|Vector2D|MakeVector2D 2.0 1.0)))
    (:then_4
      (return (LocalVariables|GetPieceConfig)))))