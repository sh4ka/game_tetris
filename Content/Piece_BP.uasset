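; Piece actor for a block-grid game that spawns a group of colored Block_BP actors from a layout of grid coordinates.
; Spawn scales each coordinate by the game mode's offsets in the X-Z plane, relative to the root, and returns the collected blocks.
; The construction script caches those offsets and builds visible 4x4 grid lines from thin, stretched cube meshes.
; GetTopMiddleVector is a stub returning zero, and the event graph is empty.
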(event EventBeginPlay)

(event Collision|EventActorBeginOverlap
  (params (OtherActor :type Actor%20Object%20Reference)))

(event EventTick
  (params (DeltaSeconds :type Float%20%28single-precision%29)))

(fn ConstructionScript
  (bind _aslppgame_mode_bp (Utilities|Casting|CastToLPPGameMode_BP (Game|GetGameMode))
    (:then
      (bind _output_get (Variables|Default|SetGameMode _aslppgame_mode_bp))
      (Variables|Default|SetVerticalOffset (Variables|/Game/LPPGameMode_BP.LPPGameMode_BP_C|GetVerticalOffset _output_get))
      (Variables|Default|SetHorizontalOffset (Variables|/Game/LPPGameMode_BP.LPPGameMode_BP_C|GetHorizontalOffset _output_get))
      (Variables|Default|SetNumColumns 4)
      (Variables|Default|SetNumRows 4))
    (:CastFailed
      _))
  (Utilities|FlowControl|Sequence
    (:then_0
      (|AddColumnCubes_2))
    (:then_1
      (|AddRowCubes_2))))

(fn Spawn
  (params (LocationConfig :type Array%20of%20Vector%202D%20Structures) (PieceColor :type Integer))
  (bind _defaultsceneroot (Variables|Default|GetDefaultSceneRoot))
  (bind _gamemode (Variables|Default|GetGameMode))
  (bind _returnvalue (Transformation|GetWorldLocation _defaultsceneroot))
  (for _array_element LocationConfig
    (bind _returnvalue_2 (Game|SpawnActorfromClass "/Game/Block_BP.Block_BP_C" (Math|Transform|MakeTransform (Math|Vector|MakeVector (+ (.x _returnvalue) (* (.x _array_element) (Variables|/Game/LPPGameMode_BP.LPPGameMode_BP_C|GetHorizontalOffset _gamemode))) 0.0 (+ (* (.y _array_element) (Variables|/Game/LPPGameMode_BP.LPPGameMode_BP_C|GetVerticalOffset _gamemode)) (.z _returnvalue))) "0, 0, 0" "1,1,1") "Undefined" 0 PieceColor 0))
    (Utilities|Array|Add (Variables|Default|GetPieces) _returnvalue_2))
  (return (Variables|Default|GetPieces)))

(fn GetTopMiddleVector
  (return ""))