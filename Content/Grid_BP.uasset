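; Grid actor that builds the bordered playfield, with side and bottom collision, entirely in its construction script.
; It copies column and row counts and spacing from LPPGameMode_BP, then places stretched cube meshes as grid lines, showing only the left, right and bottom edges.
; Hidden box components form the side and base walls, using fixed scales that do not follow the grid dimensions.
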(event EventBeginPlay)

(event Collision|EventActorBeginOverlap
  (params (OtherActor :type Actor%20Object%20Reference)))

(event EventTick
  (params (DeltaSeconds :type Float%20%28single-precision%29)))

(fn ConstructionScript
  (bind _aslppgame_mode_bp (Utilities|Casting|CastToLPPGameMode_BP (Game|GetGameMode))
    (:then
      (bind _output_get (Variables|Default|SetGameMode _aslppgame_mode_bp))
      (Variables|Default|SetVerticalOffset (Variables|/Game/LPPGameMode_BP.LPPGameMode_BP_C|GetVerticalOffset _output_get))
      (Variables|Default|SetHorizontalOffset (Variables|/Game/LPPGameMode_BP.LPPGameMode_BP_C|GetHorizontalOffset _output_get))
      (Variables|Default|SetNumColumns (Variables|/Game/LPPGameMode_BP.LPPGameMode_BP_C|GetNumColumns _output_get))
      (Variables|Default|SetNumRows (Variables|/Game/LPPGameMode_BP.LPPGameMode_BP_C|GetNumRows _output_get)))
    (:CastFailed
      _))
  (Utilities|FlowControl|Sequence
    (:then_0
      (|AddColumnCubes))
    (:then_1
      (|AddRowCubes))
    (:then_2
      (|AddColumnCollisionBoxes))
    (:then_3
      (|AddBaseCollisionBox))))