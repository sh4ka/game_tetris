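; Block actor Blueprint whose skeletal mesh takes one of seven colors chosen by an integer BlockColor.
; The construction script calls SetColorByInt, then caches the game mode cast to LPPGameMode_BP.
; SetColorByInt walks a branch chain to create a dynamic instance of the matching color material, stores it and applies it to slot 0, with yellow as the fallback.
; The event graph holds only disabled placeholder events.
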(event EventBeginPlay)

(event Collision|EventActorBeginOverlap
  (params (OtherActor :type Actor%20Object%20Reference)))

(event EventTick
  (params (DeltaSeconds :type Float%20%28single-precision%29)))

(fn ConstructionScript
  (CallFunction|SetColorbyInt (Variables|Default|GetblockColor))
  (bind _aslppgame_mode_bp (Utilities|Casting|CastToLPPGameMode_BP (Game|GetGameMode)))
  (Variables|Default|SetGameMode _aslppgame_mode_bp))

(fn SetColorbyInt
  (params (BlockColorI :type Integer))
  (bind _skeletalmesh (Variables|Default|GetSkeletalMesh))
  (if (== BlockColorI 0)
    (bind _returnvalue (Rendering|Material|CreateDynamicMaterialInstance "/Game/StaticMeshes/Materials/BlockColor_Instance_Blue.BlockColor_Instance_Blue" "None" "None" :!class /Script/Engine.KismetMaterialLibrary))
    (bind _output_get (Variables|Default|SetMyMattInst_Dyn _returnvalue))
    (Rendering|Material|SetMaterial _skeletalmesh 0 _output_get)
    (elif (== BlockColorI 1)
      (bind _returnvalue_2 (Rendering|Material|CreateDynamicMaterialInstance "/Game/StaticMeshes/Materials/BlockColor_Instance_Green.BlockColor_Instance_Green" "None" "None" :!class /Script/Engine.KismetMaterialLibrary))
      (bind _output_get_2 (Variables|Default|SetMyMattInst_Dyn _returnvalue_2))
      (Rendering|Material|SetMaterial _skeletalmesh 0 _output_get_2)
      (elif (== BlockColorI 2)
        (bind _returnvalue_3 (Rendering|Material|CreateDynamicMaterialInstance "/Game/StaticMeshes/Materials/BlockColor_Instance_Orange.BlockColor_Instance_Orange" "None" "None" :!class /Script/Engine.KismetMaterialLibrary))
        (bind _output_get_3 (Variables|Default|SetMyMattInst_Dyn _returnvalue_3))
        (Rendering|Material|SetMaterial _skeletalmesh 0 _output_get_3)
        (elif (== BlockColorI 3)
          (bind _returnvalue_4 (Rendering|Material|CreateDynamicMaterialInstance "/Game/StaticMeshes/Materials/BlockColor_Instance_Purple.BlockColor_Instance_Purple" "None" "None" :!class /Script/Engine.KismetMaterialLibrary))
          (bind _output_get_4 (Variables|Default|SetMyMattInst_Dyn _returnvalue_4))
          (Rendering|Material|SetMaterial _skeletalmesh 0 _output_get_4)
          (elif (== BlockColorI 4)
            (bind _returnvalue_5 (Rendering|Material|CreateDynamicMaterialInstance "/Game/StaticMeshes/Materials/BlockColor_Instance_Red.BlockColor_Instance_Red" "None" "None" :!class /Script/Engine.KismetMaterialLibrary))
            (bind _output_get_5 (Variables|Default|SetMyMattInst_Dyn _returnvalue_5))
            (Rendering|Material|SetMaterial _skeletalmesh 0 _output_get_5)
            (elif (== BlockColorI 5)
              (bind _returnvalue_6 (Rendering|Material|CreateDynamicMaterialInstance "/Game/StaticMeshes/Materials/BlockColor_Instance_Teal.BlockColor_Instance_Teal" "None" "None" :!class /Script/Engine.KismetMaterialLibrary))
              (bind _output_get_6 (Variables|Default|SetMyMattInst_Dyn _returnvalue_6))
              (Rendering|Material|SetMaterial _skeletalmesh 0 _output_get_6)
              (else
                (bind _returnvalue_7 (Rendering|Material|CreateDynamicMaterialInstance "/Game/StaticMeshes/Materials/BlockColor_Instance_Yellow.BlockColor_Instance_Yellow" "None" "None" :!class /Script/Engine.KismetMaterialLibrary))
                (bind _output_get_7 (Variables|Default|SetMyMattInst_Dyn _returnvalue_7))
                (Rendering|Material|SetMaterial _skeletalmesh 0 _output_get_7))))))))
  (return))