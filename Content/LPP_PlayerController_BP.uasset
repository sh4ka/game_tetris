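; Player controller for a Tetris-style falling-block game, moving the current piece using state held in LPPGameMode_BP.
; A re-armed timer and MoveDown share the fall step, while Drop speeds it up and locks sideways movement.
; Line traces per block gate movement against Grid_BP and Block_BP.
; A blocked fall counts blocks per row, destroys full rows without shifting others, then spawns the next piece; rotation is an unwired stub.
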(event Custom|FallDownOneSpace
  (bind _gamemode (Variables|Default|GetGameMode))
  (if (Variables|/Game/LPPGameMode_BP.LPPGameMode_BP_C|GetbIsQuadDroppingFaster _gamemode)
    (Variables|/Game/LPPGameMode_BP.LPPGameMode_BP_C|SetCurrentTimeBetweenFalls _gamemode (Variables|/Game/LPPGameMode_BP.LPPGameMode_BP_C|GetTimeBetweenFasterFalls _gamemode))
    (else
      (Variables|/Game/LPPGameMode_BP.LPPGameMode_BP_C|SetCurrentTimeBetweenFalls _gamemode (Variables|/Game/LPPGameMode_BP.LPPGameMode_BP_C|GetTimeBetweenAutomaticFalls _gamemode))))
  (Utilities|Time|SetTimerbyFunctionName 0 "FallDownOneSpace" (Variables|/Game/LPPGameMode_BP.LPPGameMode_BP_C|GetCurrentTimeBetweenFalls _gamemode))
  ;[1 1 1] decide what half to move down and move it
  (bind _bblocksfree (CallFunction|CanMoveDown))
  (if _bblocksfree
    (CallFunction|MoveBlocksDownOneSpace)
    (else
      (CallFunction|FinishFall))))

(event EventBeginPlay
  (bind _gamemode (Variables|Default|GetGameMode))
  (Default|SpawnNewPiece _gamemode (Variables|/Game/LPPGameMode_BP.LPPGameMode_BP_C|GetNoiseMap _gamemode))
  (Utilities|Time|SetTimerbyFunctionName 0 "FallDownOneSpace" (Variables|/Game/LPPGameMode_BP.LPPGameMode_BP_C|GetTimeBetweenAutomaticFalls _gamemode)))

(event Input|ActionEvents|InputActionRotateClockwise
  (params (Key :type Key%20Structure :default "None")))

(event Input|ActionEvents|InputActionMoveLeft
  (params (Key :type Key%20Structure :default "None"))
  (:Pressed
    (if (not (Variables|/Game/LPPGameMode_BP.LPPGameMode_BP_C|GetbIsQuadDroppingFaster (Variables|Default|GetGameMode)))
      (bind _bcanmove (CallFunction|CanMoveLeft))
      (if _bcanmove
        (CallFunction|MoveBlocksLeft)))))

(event Input|ActionEvents|InputActionRotateCounterclockwise
  (params (Key :type Key%20Structure :default "None")))

(event Input|ActionEvents|InputActionMoveRight
  (params (Key :type Key%20Structure :default "None"))
  (:Pressed
    (if (not (Variables|/Game/LPPGameMode_BP.LPPGameMode_BP_C|GetbIsQuadDroppingFaster (Variables|Default|GetGameMode)))
      (bind _bcanmove (CallFunction|CanMoveRight))
      (if _bcanmove
        (CallFunction|MoveBlocksRight)))))

(event Input|ActionEvents|InputActionMoveDown
  (params (Key :type Key%20Structure :default "None"))
  (bind _gamemode (Variables|Default|GetGameMode))
  (:Pressed
    (if (Variables|/Game/LPPGameMode_BP.LPPGameMode_BP_C|GetbIsQuadDroppingFaster _gamemode)
      (Variables|/Game/LPPGameMode_BP.LPPGameMode_BP_C|SetCurrentTimeBetweenFalls _gamemode (Variables|/Game/LPPGameMode_BP.LPPGameMode_BP_C|GetTimeBetweenFasterFalls _gamemode))
      (else
        (Variables|/Game/LPPGameMode_BP.LPPGameMode_BP_C|SetCurrentTimeBetweenFalls _gamemode (Variables|/Game/LPPGameMode_BP.LPPGameMode_BP_C|GetTimeBetweenAutomaticFalls _gamemode))))
    (Utilities|Time|SetTimerbyFunctionName 0 "FallDownOneSpace" (Variables|/Game/LPPGameMode_BP.LPPGameMode_BP_C|GetCurrentTimeBetweenFalls _gamemode))
    ;[1 1 1] decide what half to move down and move it
    (bind _bblocksfree (CallFunction|CanMoveDown))
    (if _bblocksfree
      (CallFunction|MoveBlocksDownOneSpace)
      (else
        (CallFunction|FinishFall)))))

(event Input|ActionEvents|InputActionDrop
  (params (Key :type Key%20Structure :default "None"))
  (:Pressed
    (Variables|/Game/LPPGameMode_BP.LPPGameMode_BP_C|SetbIsQuadDroppingFaster (Variables|Default|GetGameMode) true)
    (CallFunction|FallDownOneSpace)))

(fn ConstructionScript
  (bind _aslppgame_mode_bp (Utilities|Casting|CastToLPPGameMode_BP (Game|GetGameMode)))
  (Variables|Default|SetGameMode _aslppgame_mode_bp))

(fn RotateBlocksCW)

(fn RotateBlocksCCW)

(fn MoveBlocksLeft
  (for _array_element (Variables|/Game/LPPGameMode_BP.LPPGameMode_BP_C|GetCurrentPieces (Variables|Default|GetGameMode))
    (Transformation|SetActorLocation _array_element (Math|Vector|MakeVector (- (.x (Transformation|GetActorLocation _array_element)) (Variables|/Game/LPPGameMode_BP.LPPGameMode_BP_C|GetHorizontalOffset (Variables|Default|GetGameMode))) (.y (Transformation|GetActorLocation _array_element)) (.z (Transformation|GetActorLocation _array_element))) false false)))

(fn MoveBlocksRight
  (for _array_element (Variables|/Game/LPPGameMode_BP.LPPGameMode_BP_C|GetCurrentPieces (Variables|Default|GetGameMode))
    (Transformation|SetActorLocation _array_element (Math|Vector|MakeVector (+ (.x (Transformation|GetActorLocation _array_element)) (Variables|/Game/LPPGameMode_BP.LPPGameMode_BP_C|GetHorizontalOffset (Variables|Default|GetGameMode))) (.y (Transformation|GetActorLocation _array_element)) (.z (Transformation|GetActorLocation _array_element))) false false)))

(fn CanMoveLeft
  (bind _gamemode (Variables|Default|GetGameMode))
  (bind _currentpieces (Variables|/Game/LPPGameMode_BP.LPPGameMode_BP_C|GetCurrentPieces _gamemode))
  (for _array_element _currentpieces
    (bind _outhit (Collision|LineTraceForObjects (Transformation|GetActorLocation _array_element) (+ (Transformation|GetActorLocation _array_element) (Math|Vector|MakeVector (* -1 (Variables|/Game/LPPGameMode_BP.LPPGameMode_BP_C|GetHorizontalOffset _gamemode)) 0.0 0.0)) (LocalVariables|GetObjectTypes) false _currentpieces "None"))
    (Utilities|IsValid (.hitactor _outhit)
      (:Is%20Valid
        (if (or (== (Utilities|GetClass (.hitactor _outhit)) "/Game/Grid_BP.Grid_BP_C") (== (Utilities|GetClass (.hitactor _outhit)) "/Game/Block_BP.Block_BP_C"))
          (return false)))))
  (return true))

(fn CanMoveRight
  (bind _gamemode (Variables|Default|GetGameMode))
  (bind _currentpieces (Variables|/Game/LPPGameMode_BP.LPPGameMode_BP_C|GetCurrentPieces _gamemode))
  (for _array_element _currentpieces
    (bind _outhit (Collision|LineTraceForObjects (Transformation|GetActorLocation _array_element) (+ (Transformation|GetActorLocation _array_element) (Math|Vector|MakeVector (Variables|/Game/LPPGameMode_BP.LPPGameMode_BP_C|GetHorizontalOffset _gamemode) 0.0 0.0)) (LocalVariables|GetObjectTypes) false _currentpieces "None"))
    (Utilities|IsValid (.hitactor _outhit)
      (:Is%20Valid
        (if (or (== (Utilities|GetClass (.hitactor _outhit)) "/Game/Grid_BP.Grid_BP_C") (== (Utilities|GetClass (.hitactor _outhit)) "/Game/Block_BP.Block_BP_C"))
          (return false)))))
  (return true))

(fn CanMoveDown
  (bind _gamemode (Variables|Default|GetGameMode))
  (bind _currentpieces (Variables|/Game/LPPGameMode_BP.LPPGameMode_BP_C|GetCurrentPieces _gamemode))
  (LocalVariables|SetblocksCanFall 0)
  (for _array_element _currentpieces
    (bind _outhit (Collision|LineTraceForObjects (Transformation|GetActorLocation _array_element) (+ (Transformation|GetActorLocation _array_element) (Math|Vector|MakeVector 0.0 0.0 (* (Variables|/Game/LPPGameMode_BP.LPPGameMode_BP_C|GetVerticalOffset _gamemode) -1.0))) (LocalVariables|GetObjectTypes) false _currentpieces "None"))
    (Utilities|IsValid (.hitactor _outhit)
      (:Is%20Valid
        (if (or (== (Utilities|GetClass (.hitactor _outhit)) "/Game/Grid_BP.Grid_BP_C") (== (Utilities|GetClass (.hitactor _outhit)) "/Game/Block_BP.Block_BP_C"))
          ;[1 1 1] cannot fall, reset to 0
          (LocalVariables|SetblocksCanFall 0)
          (else
            ;[1 1 1] can fall, increase count
            (Math|Integer|IncrementInt (LocalVariables|GetblocksCanFall) :!label _label))))
      (:Is%20Not%20Valid
        (goto _label))))
  (return (== (LocalVariables|GetblocksCanFall) 4)))

(fn FinishFall
  (bind _gamemode (Variables|Default|GetGameMode))
  (bind _gamemode_2 (Variables|Default|GetGameMode))
  (CallFunction|CheckCompletedRows)
  (Variables|/Game/LPPGameMode_BP.LPPGameMode_BP_C|SetbIsQuadDroppingFaster _gamemode false)
  (Utilities|Time|SetTimerbyFunctionName 0 "FallDownOneSpace" (Variables|/Game/LPPGameMode_BP.LPPGameMode_BP_C|GetTimeBetweenAutomaticFalls _gamemode))
  (Default|SpawnNewPiece _gamemode_2 (Variables|/Game/LPPGameMode_BP.LPPGameMode_BP_C|GetNoiseMap _gamemode_2))
  (return))

(fn CheckCompletedRows
  (bind _rowblockcount (LocalVariables|GetrowBlockCount))
  (bind _gamemode (Variables|Default|GetGameMode))
  (bind _gamemode_2 (Variables|Default|GetGameMode))
  (bind _verticaloffset (Variables|/Game/LPPGameMode_BP.LPPGameMode_BP_C|GetVerticalOffset _gamemode))
  (bind _horizontaloffset (Variables|/Game/LPPGameMode_BP.LPPGameMode_BP_C|GetHorizontalOffset _gamemode_2))
  (Utilities|Array|Clear (Variables|Default|GetBlock%20locations))
  (bind _outactors (Actor|GetAllActorsOfClass "/Game/Block_BP.Block_BP_C"))
  (for _array_element _outactors
    (Utilities|Array|Add (Variables|Default|GetBlock%20locations) (Math|Vector2D|MakeVector2D (- (/ (+ (/ _horizontaloffset 2.0) (- (.x (.location (Transformation|GetActorTransform _array_element))) 5e+02)) _horizontaloffset) 1.0) (- (/ (+ (.z (.location (Transformation|GetActorTransform _array_element))) (/ _verticaloffset 2.0)) _verticaloffset) 1.0))))
  (for _array_element_2 (Variables|Default|GetBlock%20locations)
    (if (> (Math|Float|Truncate (.y _array_element_2)) -1)
      (Utilities|Array|SetArrayElem _rowblockcount (Math|Float|Truncate (.y _array_element_2)) (+ (Utilities|Array|Get(acopy) _rowblockcount (Math|Float|Truncate (.y _array_element_2))) 1.0))))
  (for (_array_element_3 _array_index) _rowblockcount
    (if (> _array_element_3 9.0)
      (CallFunction|RemoveBlocksinRow _array_index))))

(fn MoveBlocksDownOneSpace
  (for _array_element (Variables|/Game/LPPGameMode_BP.LPPGameMode_BP_C|GetCurrentPieces (Variables|Default|GetGameMode))
    (Transformation|SetActorLocation _array_element (Math|Vector|MakeVector (.x (Transformation|GetActorLocation _array_element)) (.y (Transformation|GetActorLocation _array_element)) (- (.z (Transformation|GetActorLocation _array_element)) (Variables|/Game/LPPGameMode_BP.LPPGameMode_BP_C|GetHorizontalOffset (Variables|Default|GetGameMode)))) false false)))

(fn RemoveBlocksinRow
  (params (Row%20Number :type Integer))
  (bind _gamemode (Variables|Default|GetGameMode))
  (bind _gamemode_2 (Variables|Default|GetGameMode))
  (bind _horizontaloffset (Variables|/Game/LPPGameMode_BP.LPPGameMode_BP_C|GetHorizontalOffset _gamemode_2))
  (bind _verticaloffset (Variables|/Game/LPPGameMode_BP.LPPGameMode_BP_C|GetVerticalOffset _gamemode))
  (bind _returnvalue (* Row%20Number _verticaloffset))
  ;[1 1 1] iterate all columns in row
  (for _index (range 0 (- (Variables|/Game/LPPGameMode_BP.LPPGameMode_BP_C|GetNumColumns _gamemode) 1))
    ;[1 1 1] detect all blocks in a given row
    (bind _outhit (Collision|LineTraceForObjects (Math|Vector|MakeVector (+ (* _index _horizontaloffset) 5e+02) 0.0 _returnvalue) (Math|Vector|MakeVector (+ (+ (* _index _horizontaloffset) 5e+02) (/ _horizontaloffset 2.0)) 0.0 (+ _returnvalue (/ _verticaloffset 2.0))) (LocalVariables|Getobject%20types) false (Utilities|Array|MakeArray (Variables|/Game/LPPGameMode_BP.LPPGameMode_BP_C|GetGrid (Variables|Default|GetGameMode))) "None"))
    (Utilities|IsValid (.hitactor _outhit)
      (:Is%20Valid
        (if (== (Utilities|GetClass (.hitactor _outhit)) "/Game/Block_BP.Block_BP_C")
          (Actor|DestroyActor (.hitactor _outhit)))))))