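; Game mode for a two-color falling-block puzzle that spawns the grid at BeginPlay and provides the 2x2 quads of blocks.
; Construction seeds the current fall interval from TimeBetweenAutomaticFalls.
; SpawnNewQuad places four Block_BP actors above the grid's horizontal middle, positioned relative to the bottom-left block, and stores them for GetQuadElements.
; DecideColorsForNewQuad randomly picks their boolean colors from a hard-coded table of solid, striped, L-shaped and diagonal patterns.
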(event EventBeginPlay
  (Game|SpawnActorfromClass "/Game/Grid_BP.Grid_BP_C" (Math|Transform|MakeTransform "0, 0, 0") "Undefined" 0 0))

(fn ConstructionScript
  (Variables|Default|SetCurrentTimeBetweenFalls (Variables|Default|GetTimeBetweenAutomaticFalls)))

(fn GetQuadElements
  (return (Utilities|Array|MakeArray (Variables|Default|GetQuad_TL) (Variables|Default|GetQuad_TR) (Variables|Default|GetQuad_BL) (Variables|Default|GetQuad_BR))))

(fn SpawnNewQuad
  (bind _colors (CallFunction|DecideColorsforNewQuad))
  (LocalVariables|SetColorsArray _colors)
  (Utilities|FlowControl|Sequence
    (:then_0
      (bind _returnvalue (Game|SpawnActorfromClass "/Game/Block_BP.Block_BP_C" (Math|Transform|MakeTransform (Math|Vector|MakeVector (* (- (Math|Conversions|ToFloat(Integer) (/ (Variables|Default|GetNumColumns) 2)) 0.5) (Variables|Default|GetHorizontalOffset)) 0.0 (* (+ (Math|Conversions|ToFloat(Integer) (Variables|Default|GetNumRows)) 0.5) (Variables|Default|GetVerticalOffset)))) "Undefined" 0 (Utilities|Array|Get(acopy) (LocalVariables|GetColorsArray)) 0))
      (Variables|Default|SetQuad_BL _returnvalue))
    (:then_1
      (bind _returnvalue_2 (Game|SpawnActorfromClass "/Game/Block_BP.Block_BP_C" (Math|Transform|MakeTransform (Math|Vector|MakeVector (.x (.location (Transformation|GetActorTransform (Variables|Default|GetQuad_BL)))) (.y (.location (Transformation|GetActorTransform (Variables|Default|GetQuad_BL)))) (+ (.z (.location (Transformation|GetActorTransform (Variables|Default|GetQuad_BL)))) (Variables|Default|GetVerticalOffset))) (.rotation (Transformation|GetActorTransform (Variables|Default|GetQuad_BL))) (.scale (Transformation|GetActorTransform (Variables|Default|GetQuad_BL)))) "Undefined" 0 (Utilities|Array|Get(acopy) (LocalVariables|GetColorsArray) 1) 0))
      (Variables|Default|SetQuad_TL _returnvalue_2))
    (:then_2
      (bind _returnvalue_3 (Game|SpawnActorfromClass "/Game/Block_BP.Block_BP_C" (Math|Transform|MakeTransform (Math|Vector|MakeVector (+ (Variables|Default|GetHorizontalOffset) (.x (.location (Transformation|GetActorTransform (Variables|Default|GetQuad_BL))))) (.y (.location (Transformation|GetActorTransform (Variables|Default|GetQuad_BL)))) (+ (.z (.location (Transformation|GetActorTransform (Variables|Default|GetQuad_BL)))) (Variables|Default|GetVerticalOffset))) (.rotation (Transformation|GetActorTransform (Variables|Default|GetQuad_BL))) (.scale (Transformation|GetActorTransform (Variables|Default|GetQuad_BL)))) "Undefined" 0 (Utilities|Array|Get(acopy) (LocalVariables|GetColorsArray) 3) 0))
      (Variables|Default|SetQuad_TR _returnvalue_3))
    (:then_3
      (bind _returnvalue_4 (Game|SpawnActorfromClass "/Game/Block_BP.Block_BP_C" (Math|Transform|MakeTransform (Math|Vector|MakeVector (+ (Variables|Default|GetHorizontalOffset) (.x (.location (Transformation|GetActorTransform (Variables|Default|GetQuad_BL))))) (.y (.location (Transformation|GetActorTransform (Variables|Default|GetQuad_BL)))) (.z (.location (Transformation|GetActorTransform (Variables|Default|GetQuad_BL))))) (.rotation (Transformation|GetActorTransform (Variables|Default|GetQuad_BL))) (.scale (Transformation|GetActorTransform (Variables|Default|GetQuad_BL)))) "Undefined" 0 (Utilities|Array|Get(acopy) (LocalVariables|GetColorsArray) 2) 0))
      (Variables|Default|SetQuad_BR _returnvalue_4))
    (:then_4
      (return))))

(fn DecideColorsforNewQuad
  (switch int (Math|Random|RandomInteger (LocalVariables|GetNumConfigurations))
    (:0
      (LocalVariables|SetColorsArray (Utilities|Array|MakeArray false false false false)) ; solid color 0
    )
    (:1
      (LocalVariables|SetColorsArray (Utilities|Array|MakeArray true true true true)) ; solid color 1
    )
    (:2
      (LocalVariables|SetColorsArray (Utilities|Array|MakeArray false false true true)) ; parallel vertical lines, color 0 on the left
    )
    (:3
      (LocalVariables|SetColorsArray (Utilities|Array|MakeArray true true false false)) ; parallel vertical lines color 1 on the left
    )
    (:4
      (LocalVariables|SetColorsArray (Utilities|Array|MakeArray true false true false)) ; parallel horizontal lines color 0 on top
    )
    (:5
      (LocalVariables|SetColorsArray (Utilities|Array|MakeArray false true false true)) ; parallel horizontal lines color 1 on top
    )
    (:6
      (LocalVariables|SetColorsArray (Utilities|Array|MakeArray true false true true)) ; l shape with color 0 at top left
    )
    (:7
      (LocalVariables|SetColorsArray (Utilities|Array|MakeArray true true true false)) ; l shape with color 0 at top right
    )
    (:8
      (LocalVariables|SetColorsArray (Utilities|Array|MakeArray false true true true)) ; l shape with color 0 at bottom left
    )
    (:9
      (LocalVariables|SetColorsArray (Utilities|Array|MakeArray true true false true)) ; l shape with color 0 at bottom right
    )
    (:10
      (LocalVariables|SetColorsArray (Utilities|Array|MakeArray false true false false)) ; l shape with color 1 at top left
    )
    (:11
      (LocalVariables|SetColorsArray (Utilities|Array|MakeArray false false false true)) ; l shape with color 1 at top right
    )
    (:12
      (LocalVariables|SetColorsArray (Utilities|Array|MakeArray true false false false)) ; l shape with color 1 at bottom left
    )
    (:13
      (LocalVariables|SetColorsArray (Utilities|Array|MakeArray false false true false)) ; l shape with color 1 at bottom right
    )
    (:14
      (LocalVariables|SetColorsArray (Utilities|Array|MakeArray false true true false)) ; diagonal 0
    )
    (:15
      (LocalVariables|SetColorsArray (Utilities|Array|MakeArray true false false true)) ; diagonal 1
    ))
  (return (LocalVariables|GetColorsArray)))