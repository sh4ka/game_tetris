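; Square piece Blueprint for a falling-block grid game, providing the logic to spawn its blocks at the top middle of the board.
; BeginPlay caches the LPP game mode, which supplies the column and row counts and cell offsets.
; AddBlock spawns a Block_BP for each grid offset in the given layout, measured from that top-middle point in the X-Z plane, and returns them collected in Quads.
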(event EventBeginPlay
  (bind _aslppgame_mode_bp (Utilities|Casting|CastToLPPGameMode_BP (Game|GetGameMode)))
  (Variables|Default|SetGameMode _aslppgame_mode_bp))

(fn ConstructionScript)

(fn AddBlock
  (params (Location%20Config :type Array%20of%20Vector%202D%20Structures))
  (bind _gamemode (Variables|Default|GetGameMode))
  (bind _location (CallFunction|GetTopMiddleVector))
  (bind _output_get (Variables|Default|SetSpawnLocation _location))
  (for _array_element Location%20Config
    (bind _returnvalue (Game|SpawnActorfromClass "/Game/Block_BP.Block_BP_C" (Math|Transform|MakeTransform (Math|Vector|MakeVector (+ (.x _output_get) (* (.x _array_element) (Variables|/Game/LPPGameMode_BP.LPPGameMode_BP_C|GetHorizontalOffset _gamemode))) 0.0 (+ (* (.y _array_element) (Variables|/Game/LPPGameMode_BP.LPPGameMode_BP_C|GetVerticalOffset _gamemode)) (.z _output_get))) "0, 0, 0" (Variables|Default|GetBlockSize)) "Undefined" 0 false 0))
    (Utilities|Array|Add (Variables|Default|Getquads) _returnvalue))
  (return (Variables|Default|Getquads)))

(fn GetTopMiddleVector
  (bind _gamemode (Variables|Default|GetGameMode))
  (bind _gamemode_2 (Variables|Default|GetGameMode))
  (return (Math|Vector|MakeVector (+ (* (- (Math|Conversions|ToFloat(Integer) (/ (Variables|/Game/LPPGameMode_BP.LPPGameMode_BP_C|GetNumColumns _gamemode) 2)) 0.5) (Variables|/Game/LPPGameMode_BP.LPPGameMode_BP_C|GetHorizontalOffset _gamemode)) 5e+02) 0.0 (* (+ (Math|Conversions|ToFloat(Integer) (Variables|/Game/LPPGameMode_BP.LPPGameMode_BP_C|GetNumRows _gamemode_2)) 0.5) (Variables|/Game/LPPGameMode_BP.LPPGameMode_BP_C|GetVerticalOffset _gamemode_2)))))